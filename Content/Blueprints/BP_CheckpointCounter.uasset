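; BP_CheckpointCounter is a checkpoint actor that counts and displays the actors that have touched its static mesh.
; Each overlapping actor is added uniquely to a Players array, with no check yet that it is a player.
; The array's RepNotify refreshes a text render with the count and prints debug messages.
; The construction script also runs that text update to set the initial display.
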(event OnComponentBeginOverlap(StaticMesh)
  (params (OtherActor :type Actor%20Object%20Reference) (OtherComp :type Primitive%20Component%20Object%20Reference) (OtherBodyIndex :type Integer) (bFromSweep :type Boolean) (SweepResult :type Hit%20Result%20Structure%20%28by%20ref%29))
  ;[1 1 1] todo: make sure other actor is a player
  (Utilities|Array|AddUnique (Variables|Default|GetPlayers) OtherActor))

(fn ConstructionScript
  (CallFunction|UpdateTextRender))

(fn UpdateTextRender
  (bind _players (Variables|Default|GetPlayers))
  (bind _returnvalue (Utilities|Array|Length _players))
  (bind _returnvalue_2 (Utilities|String|BuildString(Integer) "Num players: " "" _returnvalue))
  (Development|PrintString _returnvalue_2)
  (Rendering|Components|TextRender|SetText (Variables|Default|GetTextRender) _returnvalue_2))

(fn OnRepPlayers
  (Development|PrintString "Players updated")
  (CallFunction|UpdateTextRender))