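; BP_SpeedPickup is a pickup actor with a hovering static mesh, named for a speed effect that is not implemented yet.
; The construction script places the mesh at InitialRelativeLocation, and a timeline started on BeginPlay offsets its Z by a curve value times HoverScale.
; The capsule overlap event only reaches an authority switch with nothing wired after it, and a player movement component lookup is left unconnected.
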(event OnComponentBeginOverlap(Capsule)
  (params (OtherActor :type Actor%20Object%20Reference) (OtherComp :type Primitive%20Component%20Object%20Reference) (OtherBodyIndex :type Integer) (bFromSweep :type Boolean) (SweepResult :type Hit%20Result%20Structure%20%28by%20ref%29))
  (Networking|SwitchHasAuthority))

(event EventBeginPlay
  (bind _initialrelativelocation (Variables|Default|GetInitialRelativeLocation))
  (bind _zvalue (Timeline|HoverTimeline Play)
    (:Update
      (Transformation|SetRelativeLocation (Variables|Default|GetStaticMesh) (Math|Vector|MakeVector (.x _initialrelativelocation) (.y _initialrelativelocation) (+ (.z _initialrelativelocation) (* _zvalue (Variables|Default|GetHoverScale)))) false))))

(event EventActorBeginOverlap
  (params (OtherActor :type Actor%20Object%20Reference)))

(event EventTick
  (params (DeltaSeconds :type Float%20%28single-precision%29)))

(fn ConstructionScript
  (Transformation|SetRelativeLocation (Variables|Default|GetStaticMesh) (Variables|Default|GetInitialRelativeLocation) false))