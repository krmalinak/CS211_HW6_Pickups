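; BP_Landmine is a networked landmine that explodes when a pawn overlaps its sphere.
; On the server, only player pawn 0 triggers Explode, while remote copies spawn explosion particles on any overlap.
; Explode plays effects, then, only if the overlapping actor is a NetworkedVRChar, applies authority-only radial falloff damage and destroys the mine.
; BeginPlay hard-codes player pawn 1 as Instigator, and debug prints remain.
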(event OnComponentBeginOverlap(Sphere)
  (params (OtherActor :type Actor%20Object%20Reference) (OtherComp :type Primitive%20Component%20Object%20Reference) (OtherBodyIndex :type Integer) (bFromSweep :type Boolean) (SweepResult :type Hit%20Result%20Structure%20%28by%20ref%29))
  (Networking|SwitchHasAuthority
    (:Authority
      (Development|PrintString "server")
      (if (== OtherActor (Game|Player|GetPlayerPawn 0))
        (Development|PrintString "derp")
        (CallFunction|Explode)))
    (:Remote
      (Effects|SpawnEmitteratLocation "/Game/StarterContent/Particles/P_Explosion.P_Explosion" (Transformation|GetActorLocation)))))

(event Custom|Explode
  (params (HitActor :type Networked%20VR%20Char%20Object%20Reference))
  (bind _returnvalue (Transformation|GetActorLocation))
  (Effects|SpawnEmitteratLocation "/Game/StarterContent/Particles/P_Explosion.P_Explosion" _returnvalue)
  (Audio|PlaySoundatLocation "/Game/StarterContent/Audio/Explosion01.Explosion01" _returnvalue)
  (bind _asnetworked_vrchar (Utilities|Casting|CastToNetworkedVRChar (stale OnComponentBeginOverlap(Sphere) OtherActor)))
  (CallFunction|ApplyMyDamage _asnetworked_vrchar (Variables|DamageSettings|GetBaseDamage))
  (Actor|DestroyActor))

(event EventApplyMyDamage
  (params (DamagedActor :type Actor%20Object%20Reference) (BaseDamage :type Float%20%28single-precision%29))
  (Networking|SwitchHasAuthority
    (:Authority
      (Class|GameplayStatics|ApplyRadialDamagewithFalloff (Variables|DamageSettings|GetBaseDamage) (Variables|DamageSettings|GetMinimumDamage) (Transformation|GetActorLocation) 0.0 (Variables|DamageSettings|GetDamageRadius) 2.0 "/Game/Blueprints/DT_Explosion.DT_Explosion_C" 0 self (Game|GetInstigatorController) "ECC_Visibility"))))

(event EventBeginPlay
  (Variables|Actor|SetInstigator (Game|Player|GetPlayerPawn 1)))

(fn ConstructionScript)