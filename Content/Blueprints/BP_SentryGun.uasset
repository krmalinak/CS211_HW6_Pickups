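; Sentry gun that sweeps its barrel back and forth and fires projectiles at whatever its line of sight hits.
; After a warmup delay, a timeline drives the swivel and scan mode switches on.
; Server-only Tick traces along the Arrow on the Visibility channel, firing on any hit without target filtering.
; Firing spawns BP_SentryGunProjectile ahead of the Arrow and suspends scanning for a cooldown, while the swivel resumes immediately.
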(event Custom|FireProjectile
  (bind _arrow (Variables|Default|GetArrow))
  (CallFunction|ToggleScanMode)
  (Development|PrintString "Firing projectile")
  (Game|SpawnActorfromClass "/Game/Blueprints/BP_SentryGunProjectile.BP_SentryGunProjectile_C" (Math|Transform|MakeTransform (+ (Transformation|GetWorldLocation _arrow) (* (Math|Vector|GetForwardVector _arrow) (Variables|Default|GetProjectileSpawnOffset))) (Transformation|GetWorldRotation _arrow)) true 0)
  (Utilities|FlowControl|Delay (Variables|Default|GetCoolDownTime))
  (CallFunction|ToggleScanMode))

(event EventBeginPlay
  (bind _swivelhalfrange (Variables|Default|GetSwivelHalfRange))
  (Utilities|FlowControl|Delay (Variables|Default|GetWarmupTime))
  (CallFunction|ToggleScanMode)
  (bind _swivelvalue (Timeline|SwivelTimeline Play)
    (:Update
      (Transformation|SetRelativeRotation (Variables|Default|GetBarrel) (Math|Rotator|MakeRotator 9e+01 0.0 (Math|Float|Lerp (* _swivelhalfrange -1.0) _swivelhalfrange _swivelvalue)) false))))

(event EventTick
  (params (DeltaSeconds :type Float%20%28single-precision%29))
  (bind _arrow (Variables|Default|GetArrow))
  (bind _swivelhalfrange (Variables|Default|GetSwivelHalfRange))
  (bind _returnvalue (Transformation|GetWorldLocation _arrow))
  (Networking|SwitchHasAuthority
    (:Authority
      (if (Variables|Default|GetScanMode)
        (bind (_outhit _returnvalue_2) (Collision|LineTraceByChannel _returnvalue (+ _returnvalue (* (Math|Vector|GetForwardVector _arrow) (Variables|Default|GetLaserRange))) "TraceTypeQuery1" false 0 "ForOneFrame"))
        (if _returnvalue_2
          (Development|PrintString (Utilities|String|Append "Located Target: " (Utilities|GetDisplayName (.HitActor (Collision|BreakHitResult _outhit)))))
          (Utilities|FlowControl|Sequence
            (:then_0
              (bind _swivelvalue (Timeline|SwivelTimeline Stop)
                (:Update
                  (Transformation|SetRelativeRotation (Variables|Default|GetBarrel) (Math|Rotator|MakeRotator 9e+01 0.0 (Math|Float|Lerp (* _swivelhalfrange -1.0) _swivelhalfrange _swivelvalue)) false))))
            (:then_1
              (Networking|SwitchHasAuthority
                (:Authority
                  (CallFunction|FireProjectile)
                  (Timeline|SwivelTimeline Play))))))))))

(fn ConstructionScript)

(fn ToggleScanMode
  (Variables|Default|SetScanMode (not (Variables|Default|GetScanMode))))